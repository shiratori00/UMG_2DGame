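; Player controller for the Invader game, which plays inside a UMG widget with the player as a child widget.
; On BeginPlay it creates the main Invader widget, adds it to the viewport and sets Game and UI input mode.
; Movement axes move the player widget, scaled by frame time with the forward axis inverted.
; Shot fires from the player widget, or calls EnterStart on the main widget when the player cast fails.
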(event EventBeginPlay
  (bind _returnvalue (UserInterface|CreateWidget "/Game/Blueptints/Invader/WG_Main_Invader.WG_Main_Invader_C"))
  (bind _output_get (Variables|Default|SetWG_Main _returnvalue))
  (UserInterface|Viewport|AddtoViewport _output_get 0)
  (Input|SetInputModeGameandUI self 0 "DoNotLock" true))

(event EventTick
  (params (DeltaSeconds :type Float%20%28single-precision%29)))

(event Input|ActionEvents|InputActionShot
  (params (Key :type Key%20Structure))
  (:Pressed
    (bind _aswg_player_invader (Utilities|Casting|CastToWG_Player_Invader (Variables|/Game/Blueptints/Invader/WG_Main_Invader.WG_Main_Invader_C|GetPlayer (Variables|Default|GetWG_Main)))
      (:then
        (Default|Shot _aswg_player_invader))
      (:CastFailed
        (Default|EnterStart (Variables|Default|GetWG_Main))))))

(event Input|AxisEvents|InputAxisMoveRight
  (params (AxisValue :type Float%20%28single-precision%29))
  (bind _wg_main (Variables|Default|GetWG_Main))
  (bind _player (Variables|/Game/Blueptints/Invader/WG_Main_Invader.WG_Main_Invader_C|GetPlayer _wg_main))
  (Utilities|IsValid _player
    (:Is%20Valid
      (Class|MyObjectBaseWidget|Move _player (* AxisValue 1e+02 (Utilities|Time|GetWorldDeltaSeconds)) 0.0))))

(event Input|AxisEvents|InputAxisMoveForward
  (params (AxisValue :type Float%20%28single-precision%29))
  (bind _wg_main (Variables|Default|GetWG_Main))
  (bind _player (Variables|/Game/Blueptints/Invader/WG_Main_Invader.WG_Main_Invader_C|GetPlayer _wg_main))
  (Utilities|IsValid _player
    (:Is%20Valid
      (Class|MyObjectBaseWidget|Move _player 0.0 (* AxisValue 1e+02 (Utilities|Time|GetWorldDeltaSeconds) -1.0)))))

(fn ConstructionScript)