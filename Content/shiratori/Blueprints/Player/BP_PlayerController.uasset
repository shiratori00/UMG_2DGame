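; BP_PlayerController is a player controller that drives a widget-based game, forwarding movement and jump input to UMG widgets instead of a pawn.
; Init stores the main widget, initializes its map, adds it to the viewport and caches its player widget.
; The MoveRight axis calls Move on the main widget, while Jump presses call Jump on the player widget, each guarded by a validity check.
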(event EventBeginPlay)

(event EventTick
  (params (DeltaSeconds :type Float%20%28single-precision%29)))

(event Input|ActionEvents|InputActionJump
  (params (Key :type Key%20Structure))
  (bind _wg_player (Variables|Default|GetWG_Player))
  (:Pressed
    (Utilities|IsValid _wg_player
      (:Is%20Valid
        (Default|Jump _wg_player)))))

(event Input|AxisEvents|InputAxisMoveRight
  (params (AxisValue :type Float%20%28single-precision%29))
  (bind _wg_main (Variables|Default|GetWG_Main))
  (Utilities|IsValid _wg_main
    (:Is%20Valid
      (Default|Move _wg_main AxisValue))))

(fn ConstructionScript)

(fn Init
  (params (wg_Main :type WG%20Main%20Object%20Reference))
  (bind _output_get (Variables|Default|SetWG_Main wg_Main))
  (Default|InitializeMap _output_get)
  (UserInterface|Viewport|AddtoViewport (Variables|Default|GetWG_Main) 0)
  (Variables|Default|SetWG_Player (Variables|/Game/shiratori/Blueprints/Main/WG_Main.WG_Main_C|GetPlayer (Variables|Default|GetWG_Main))))